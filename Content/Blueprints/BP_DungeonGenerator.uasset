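; Procedural dungeon generator actor that builds a level at BeginPlay from a start room, random rooms and a boss room.
; A looping timer attaches random rooms at random open exits until the spawn count is met, pooling each new room's exits.
; Overlap-box checks destroy colliding rooms and wall those exits.
; Boss placement retries similarly, then walls fill remaining exits; shop placement exists but is never called here.
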(event `self.ReceiveBeginPlay`
  (bind (_returnvalue_location _returnvalue_rotation) (`KismetMathLibrary.BreakTransform` (`SceneComponent.K2_GetComponentToWorld` (`self.DefaultSceneRoot`))))
  ;[0 1 0.6343] Beginplay
  ;;[1 1 1] create wall behind start.
  (`|SpawnActorFromClass` "/Game/Blueprints/DungeonRooms/BP_FillExitsWall.BP_FillExitsWall_C" (`KismetMathLibrary.MakeTransform` _returnvalue_location _returnvalue_rotation (0.85 0.85 0.85)) "AlwaysSpawn" "MultiplyWithRoot" null null)
  (`ActorComponent.K2_DestroyComponent` (`self.ChildActor`))
  (`self.GenerateSpawnRoom`)
  (set `self.LeftToSpawn` (- (`self.SpawnAmount`) 1))
  (`self.GenerateDungeon`))

(event `TrySpawnShop`
  (bind _spawned_ (`self.GenerateShopRoom`))
  (if _spawned_
    _))

(event `GenerateDungeon`
  ;[1 0 0.6217] Generate rest of rooms
  (bind _returnvalue (`KismetSystemLibrary.K2_SetTimerDelegate` (delegate `SpawnRooms`) 0.1 true true)))

(event `SpawnRooms`
  ;[1 0 0.6217] Generate rest of rooms
  (if (>= (`self.LeftToSpawn`) 1)
    (`self.SpawnNextRoom`)
    (else
      (`KismetSystemLibrary.K2_ClearAndInvalidateTimerHandle` (stale `GenerateDungeon` _returnvalue))
      (`KismetSystemLibrary.Delay` 0.2)
      (bind _returnvalue (`KismetSystemLibrary.K2_SetTimerDelegate` (delegate `TrySpawnBoss`) 0.1 true true)))))

(event `TrySpawnBoss`
  ;[1 0 0.6217] Generate rest of rooms
  (bind _spawned_ (`self.GenerateBossRoom`))
  (if _spawned_
    (`KismetSystemLibrary.K2_ClearAndInvalidateTimerHandle` (stale `SpawnRooms` _returnvalue))
    (`self.FillDungeonExits`)))

(event `FillDungeonExits`
  ;[1 0 0.882] Spawns wall actors at exits
  (for _array_element (`self.Exits list`)
    (bind (_returnvalue_location _returnvalue_rotation _returnvalue_scale) (`KismetMathLibrary.BreakTransform` (`SceneComponent.K2_GetComponentToWorld` _array_element)))
    (`|SpawnActorFromClass` "/Game/Blueprints/DungeonRooms/BP_FillExitsWall.BP_FillExitsWall_C" (`KismetMathLibrary.MakeTransform` _returnvalue_location _returnvalue_rotation _returnvalue_scale) "AlwaysSpawn" "MultiplyWithRoot" null null)))

(event `SpawnNextRoom`
  (bind (_returnvalue_location _returnvalue_rotation _returnvalue_scale) (`KismetMathLibrary.BreakTransform` (`SceneComponent.K2_GetComponentToWorld` (`self.SelectedExitPoint`))))
  ;[1 0 0.882] SpawnRooms
  ;;[0.9249 1 0.9578] Spawn Next room
  (bind _output_get (set `self.SelectedExitPoint` (`KismetArrayLibrary.Array_Random` (`self.Exits list`))))
  (`/Engine/EditorBlueprintResources/StandardMacros.IsValid` _output_get
    (:`Is Valid`
      (bind (_returnvalue_location_2 _returnvalue_rotation_2) (`KismetMathLibrary.BreakTransform` (`SceneComponent.K2_GetComponentToWorld` _output_get)))
      (bind _returnvalue (`|SpawnActorFromClass` (`KismetArrayLibrary.Array_Random` (`self.RoomsList`)) (`KismetMathLibrary.MakeTransform` _returnvalue_location_2 _returnvalue_rotation_2) "AlwaysSpawn" "MultiplyWithRoot" null null))
      (bind _output_get_2 (set `self.LatestRoom` _returnvalue))
      (if (`KismetArrayLibrary.Array_IsEmpty` (`PrimitiveComponent.GetOverlappingComponents` (`/Game/Blueprints/DungeonRooms/BP_RoomBase.OverlapBox` _output_get_2)))
        ;;[1 1 1] adds new exits of room to list of available exits.
        (`KismetArrayLibrary.Array_Append` (`self.Exits list`) (`SceneComponent.GetChildrenComponents` (`/Game/Blueprints/DungeonRooms/BP_RoomBase.Exits` (`self.LatestRoom`)) false))
        ;;[1 1 1] Removes the recent spawned location to prevent spawning another room there
        (`KismetArrayLibrary.Array_RemoveItem` (`self.Exits list`) (`self.SelectedExitPoint`))
        (set `self.LeftToSpawn` (- (`self.LeftToSpawn`) 1))
        (else
          (`|SpawnActorFromClass` "/Game/Blueprints/DungeonRooms/BP_FillExitsWall.BP_FillExitsWall_C" (`KismetMathLibrary.MakeTransform` _returnvalue_location _returnvalue_rotation _returnvalue_scale) "AlwaysSpawn" "MultiplyWithRoot" null null) ; spawn wall to block of exit
          ;;[1 1 1] Removes the recent spawned location to prevent spawning another room there
          (`KismetArrayLibrary.Array_RemoveItem` (`self.Exits list`) (`self.SelectedExitPoint`))
          (`self.K2_DestroyActor` (`self.LatestRoom`)))))))

(fn `Add overlapping rooms to list`
  (`KismetArrayLibrary.Array_Append` (`self.OverlappingList`) (`PrimitiveComponent.GetOverlappingComponents` (`/Game/Blueprints/DungeonRooms/BP_RoomBase.OverlapBox` (`self.LatestRoom`)))))

(fn `GenerateBossRoom`
  (returns (`spawned?` :type Boolean))
  (bind (_returnvalue_location _returnvalue_rotation _returnvalue_scale) (`KismetMathLibrary.BreakTransform` (`SceneComponent.K2_GetComponentToWorld` (`self.SelectedExitPoint`))))
  (bind _output_get (set `self.SelectedExitPoint` (`KismetArrayLibrary.Array_Random` (`self.Exits list`))))
  (`/Engine/EditorBlueprintResources/StandardMacros.IsValid` _output_get
    (:`Is Valid`
      (bind (_returnvalue_location_2 _returnvalue_rotation_2) (`KismetMathLibrary.BreakTransform` (`SceneComponent.K2_GetComponentToWorld` _output_get)))
      (bind _returnvalue (`|SpawnActorFromClass` (`self.BossRoom`) (`KismetMathLibrary.MakeTransform` _returnvalue_location_2 _returnvalue_rotation_2) "AlwaysSpawn" "MultiplyWithRoot" null null))
      (bind _output_get_2 (set `self.LatestRoom` _returnvalue))
      (if (`KismetArrayLibrary.Array_IsEmpty` (`PrimitiveComponent.GetOverlappingComponents` (`/Game/Blueprints/DungeonRooms/BP_RoomBase.OverlapBox` _output_get_2)))
        ;[1 1 1] Removes the recent spawned location to prevent spawning another room there
        (`KismetArrayLibrary.Array_RemoveItem` (`self.Exits list`) (`self.SelectedExitPoint`))
        (return true)
        (else
          (`|SpawnActorFromClass` "/Game/Blueprints/DungeonRooms/BP_FillExitsWall.BP_FillExitsWall_C" (`KismetMathLibrary.MakeTransform` _returnvalue_location _returnvalue_rotation _returnvalue_scale) "AlwaysSpawn" "MultiplyWithRoot" null null) ; spawn wall to block of exit
          ;[1 1 1] Removes the recent spawned location to prevent spawning another room there
          (`KismetArrayLibrary.Array_RemoveItem` (`self.Exits list`) (`self.SelectedExitPoint`))
          (`self.K2_DestroyActor` (`self.LatestRoom`))
          (return false))))))

(fn `GenerateShopRoom`
  (returns (`spawned?` :type Boolean))
  (bind (_returnvalue_location _returnvalue_rotation _returnvalue_scale) (`KismetMathLibrary.BreakTransform` (`SceneComponent.K2_GetComponentToWorld` (`self.SelectedExitPoint`))))
  (bind _output_get (set `self.SelectedExitPoint` (`KismetArrayLibrary.Array_Random` (`self.Exits list`))))
  (`/Engine/EditorBlueprintResources/StandardMacros.IsValid` _output_get
    (:`Is Valid`
      (bind (_returnvalue_location_2 _returnvalue_rotation_2) (`KismetMathLibrary.BreakTransform` (`SceneComponent.K2_GetComponentToWorld` _output_get)))
      (bind _returnvalue (`|SpawnActorFromClass` "/Game/Blueprints/DungeonRooms/BP_ShopRoom.BP_ShopRoom_C" (`KismetMathLibrary.MakeTransform` _returnvalue_location_2 _returnvalue_rotation_2) "AlwaysSpawn" "MultiplyWithRoot" null null))
      (bind _output_get_2 (set `self.LatestRoom` _returnvalue))
      (if (`KismetArrayLibrary.Array_IsEmpty` (`PrimitiveComponent.GetOverlappingComponents` (`/Game/Blueprints/DungeonRooms/BP_RoomBase.OverlapBox` _output_get_2)))
        ;[1 1 1] Removes the recent spawned location to prevent spawning another room there
        (`KismetArrayLibrary.Array_RemoveItem` (`self.Exits list`) (`self.SelectedExitPoint`))
        (return true)
        (else
          (`|SpawnActorFromClass` "/Game/Blueprints/DungeonRooms/BP_FillExitsWall.BP_FillExitsWall_C" (`KismetMathLibrary.MakeTransform` _returnvalue_location _returnvalue_rotation _returnvalue_scale) "AlwaysSpawn" "MultiplyWithRoot" null null) ; spawn wall to block of exit
          ;[1 1 1] Removes the recent spawned location to prevent spawning another room there
          (`KismetArrayLibrary.Array_RemoveItem` (`self.Exits list`) (`self.SelectedExitPoint`))
          (`self.K2_DestroyActor` (`self.LatestRoom`))
          (return false))))))

(fn `GenerateSpawnRoom`
  ;[1 1 1] Comment
  (bind _returnvalue (`|SpawnActorFromClass` "/Game/Blueprints/DungeonRooms/BP_StartRoom.BP_StartRoom_C" (`SceneComponent.K2_GetComponentToWorld` (`self.DefaultSceneRoot`)) "AlwaysSpawn" "MultiplyWithRoot" null null))
  (`KismetArrayLibrary.Array_Append` (`self.Exits list`) (`SceneComponent.GetChildrenComponents` (`/Game/Blueprints/DungeonRooms/BP_RoomBase.Exits` _returnvalue) false)))

(fn `UserConstructionScript`)