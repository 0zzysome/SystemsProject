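; Component that spawns random loot actors at its child components' transforms, which act as spawn points.
; One second after BeginPlay, so rooms deleted for colliding spawn nothing, it shuffles the children if spawning is enabled.
; It fills either a fixed or random number of points, picking each actor class randomly from LootToSpawn.
; Missing children or too few valid points print an error.
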(event `self.ReceiveBeginPlay`
  (bind _returnvalue (`KismetMathLibrary.RandomIntegerInRange` (`self.MinSpawnAmount`) (`self.SpawnAmount`)))
  ;[1 1 1] Go through checks
  (`KismetSystemLibrary.Delay` 1.0) ; delay so they dont spawn if the room collided and got deleted
  (if (`self.bShouldSpawnLoot?`)
    (bind _output_get (set `self.Children` (`self.GetChildrenComponents` false)))
    (if (`KismetArrayLibrary.Array_IsNotEmpty` _output_get)
      (`KismetArrayLibrary.Array_Shuffle` _output_get) ; Randomize what order spawn points are in
      (if (`self.Should Random Spawn`)
        ;[1 0 0.882] Get a random number over 0 (random)
        (if (not (<= _returnvalue 0))
          (for _index (range _returnvalue)
            (bind _output (`|GetArrayItem` (`self.Children`) _index))
            ;[0 1 0.1032] spawn loot
            (`/Engine/EditorBlueprintResources/StandardMacros.IsValid` _output
              (:`Is Valid`
                (`|SpawnActorFromClass` (`KismetArrayLibrary.Array_Random` (`self.LootToSpawn`)) (`self.K2_GetComponentToWorld` _output) "Undefined" "MultiplyWithRoot" null null))
              (:`Is Not Valid`
                ;[1 1 1] Error code
                (`KismetSystemLibrary.PrintString` (`KismetStringLibrary.Concat_StrStr` "NOT ENOUGHT SPAWN POINTS TO SPAWN LOOT IN: " (`KismetSystemLibrary.GetDisplayName` (`self.GetOwner`))) :!label _label)))))
        (else
          ;[0 1 0.6343] loop fixed amount of times
          (for _index_2 (range (`self.SpawnAmount`))
            (bind _output_2 (`|GetArrayItem` (`self.Children`) _index_2))
            ;[0 1 0.1032] Spawn Loot
            (`/Engine/EditorBlueprintResources/StandardMacros.IsValid` _output_2
              (:`Is Valid`
                (`|SpawnActorFromClass` (`KismetArrayLibrary.Array_Random` (`self.LootToSpawn`)) (`self.K2_GetComponentToWorld` _output_2) "Undefined" "MultiplyWithRoot" null null))
              (:`Is Not Valid`
                (goto _label))))))
      (else
        (`KismetSystemLibrary.PrintString` "NO CHILDREN FOR LOOT SPAWNER ")))))