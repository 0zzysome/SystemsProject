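; Base boss enemy that drives its AI through a blackboard State and uses weapon and health components.
; The first DealDamage call activates chase and broadcasts BossActivated.
; AttackTrigger overlaps switch between attack and chase, while the behavior tree calls CallAttack for a random weapon attack.
; Death grants player XP and destroys weapon and boss; sight-based chase, its lost-sight timer and attack-duration setup are unconnected.
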(event `self.ReceiveBeginPlay`
  (`/Game/Blueprints/BP_WeaponComponent.CreateDefaultWeapon` (`self.BP_WeaponComponent`))
  (add `/Game/Blueprints/BP_HealthComponent.HasDied` (`self.BP_HealthComponent`) (delegate `HasDied_Event`))
  (`BlackboardComponent.SetValueAsVector` (`AIBlueprintHelperLibrary.GetBlackboard` null) "PatrolLocation" (`SceneComponent.K2_GetComponentLocation` (`self.CapsuleComponent`))))

(event `HasDied_Event`
  ;[1 1 1] Die funtions
  (bind _asbp_main_character (cast `/Game/Blueprints/BP_MainCharacter` (`GameplayStatics.GetPlayerCharacter` 0)))
  (`/Game/Blueprints/BP_MainCharacter.AddXp` _asbp_main_character 5)
  (`/Game/Blueprints/BP_WeaponComponent.DestroyWeapon` (`self.BP_WeaponComponent`))
  (`self.K2_DestroyActor`))

(event `Activate Boss`
  (`/Engine/EditorBlueprintResources/StandardMacros.IsValid` self
    (:`Is Valid`
      (`BlackboardComponent.SetValueAsEnum` (`AIBlueprintHelperLibrary.GetBlackboard` null) "State" (enumliteral `/Game/Blueprints/Enemies/E_AIState` "NewEnumerator1"))
      (`self.BossActivated`))))

(event `self.DealDamage`
  (params (DamageAmount :type "Float (double-precision)"))
  (`/Game/Blueprints/BP_HealthComponent.TakeDamageEvent` (`self.BP_HealthComponent`) DamageAmount)
  (`/Engine/EditorBlueprintResources/StandardMacros.DoOnce` false
    (:`Completed`
      (`self.Activate Boss`))))

(event `LostSightOfplayer`
  ;[1 1 1] After not getting can se player event for  time sets state to patrol
  (`BlackboardComponent.SetValueAsEnum` (`AIBlueprintHelperLibrary.GetBlackboard` null) "State" (enumliteral `/Game/Blueprints/Enemies/E_AIState` "NewEnumerator0")))

(event `self.CallAttack`
  ;[1 1 1] Attack from behavior tree to component
  (`/Game/Blueprints/BP_WeaponComponent.Attack` (`self.BP_WeaponComponent`) (`KismetArrayLibrary.Array_Random` (`self.AttackTypes`))))

(event `self.AttackTrigger.OnComponentBeginOverlap`
  (params (OverlappedComponent :type "PrimitiveComponent Object Reference") (OtherActor :type "Actor Object Reference") (OtherComp :type "PrimitiveComponent Object Reference") (OtherBodyIndex :type Integer) (bFromSweep :type Boolean) (SweepResult :type "HitResult Structure (by ref)"))
  ;[1 1 1] attack when player is in front
  (if (== OtherActor (`GameplayStatics.GetPlayerCharacter` 0))
    (set `self.Other Actor` OtherActor)
    (`BlackboardComponent.SetValueAsEnum` (`AIBlueprintHelperLibrary.GetBlackboard` null) "State" (enumliteral `/Game/Blueprints/Enemies/E_AIState` "NewEnumerator2"))
    (if (`KismetSystemLibrary.K2_IsTimerActiveHandle` (`self.ChasePlayerTimer`))
      (`KismetSystemLibrary.K2_ClearAndInvalidateTimerHandle` (`self.ChasePlayerTimer`)) ; reset timer
    )))

(event `self.AttackTrigger.OnComponentEndOverlap`
  (params (OverlappedComponent :type "PrimitiveComponent Object Reference") (OtherActor :type "Actor Object Reference") (OtherComp :type "PrimitiveComponent Object Reference") (OtherBodyIndex :type Integer))
  (bind _returnvalue (`AIBlueprintHelperLibrary.GetBlackboard` null))
  ;[1 1 1] stop attaking when player leaves
  (if (== OtherActor (`self.Other Actor`))
    (`/Engine/EditorBlueprintResources/StandardMacros.IsValid` _returnvalue
      (:`Is Valid`
        (`BlackboardComponent.SetValueAsEnum` _returnvalue "State" (enumliteral `/Game/Blueprints/Enemies/E_AIState` "NewEnumerator1"))))))

(fn `UserConstructionScript`)