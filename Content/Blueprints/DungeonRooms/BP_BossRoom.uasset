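; Dungeon boss room that spawns a boss, runs the fight trigger and opens the way to the next floor.
; After a short delay, so failed rooms get no boss, it spawns BP_BossBase and a closing wall that references it.
; The player entering the trigger activates the boss once.
; A bound health-component death event spawns the exit door, shows the next-floor text and hides the static mesh.
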(event `self.ReceiveBeginPlay`
  (bind _bossspawn (`self.BossSpawn`))
  (bind (_returnvalue_location _returnvalue_rotation _returnvalue_scale) (`KismetMathLibrary.BreakTransform` (`SceneComponent.K2_GetComponentToWorld` (`self.DefaultSceneRoot`))))
  (`parent.ReceiveBeginPlay`)
  (`SceneComponent.SetVisibility` (`self.NextFloorText`) false false)
  (`KismetSystemLibrary.Delay` 0.5) ; prevents failed rooms from spawning a boss
  ;[1 1 1] Spawn boss
  (`/Engine/EditorBlueprintResources/StandardMacros.IsValid` _bossspawn
    (:`Is Valid`
      (bind _returnvalue (`AIBlueprintHelperLibrary.SpawnAIFromClass` "/Game/Blueprints/Enemies/BP_BossBase.BP_BossBase_C" null (`SceneComponent.K2_GetComponentLocation` _bossspawn) (`SceneComponent.K2_GetComponentRotation` _bossspawn) false null))
      (bind _asbp_boss_base (cast `/Game/Blueprints/Enemies/BP_BossBase` _returnvalue))
      (bind _output_get (set `self.BossRef` _asbp_boss_base))
      (add `/Game/Blueprints/BP_HealthComponent.HasDied` (`/Game/Blueprints/Enemies/BP_BossBase.BP_HealthComponent` _output_get) (`|CreateDelegate` :!event `BossDies`))
      ;[1 1 1] Spawn wall that closes room
      (bind _returnvalue_2 (`|SpawnActorFromClass` "/Game/Blueprints/DungeonRooms/BP_BossWall.BP_BossWall_C" (`KismetMathLibrary.MakeTransform` _returnvalue_location _returnvalue_rotation _returnvalue_scale) "AlwaysSpawn" "MultiplyWithRoot" null (`self.BossRef`) null)) ; spawn wall to block of exit
      (set `self.Close Room Wall` _returnvalue_2))))

(event `self.ActivateBossTrigger.OnComponentBeginOverlap`
  (params (OverlappedComponent :type "PrimitiveComponent Object Reference") (OtherActor :type "Actor Object Reference") (OtherComp :type "PrimitiveComponent Object Reference") (OtherBodyIndex :type Integer) (bFromSweep :type Boolean) (SweepResult :type "HitResult Structure (by ref)"))
  ;[1 1 1] MAke trigger start boss fight.
  (if (== OtherActor (`GameplayStatics.GetPlayerCharacter` 0))
    (`/Engine/EditorBlueprintResources/StandardMacros.DoOnce` false
      (:`Completed`
        (`/Game/Blueprints/Enemies/BP_BossBase.Activate Boss` (`self.BossRef`))))))

(event `BossDies`
  ;[1 1 1] Spawn exit to next floor
  (`|SpawnActorFromClass` "/Game/Blueprints/BP_ExitDoor.BP_ExitDoor_C" (`SceneComponent.K2_GetComponentToWorld` (`self.ExitSpawn`)) "Undefined" "MultiplyWithRoot" null null)
  (`SceneComponent.SetVisibility` (`self.NextFloorText`) true false)
  (`SceneComponent.SetVisibility` (`self.StaticMesh`) false false))

(fn `UserConstructionScript`
  (`parent.UserConstructionScript`))