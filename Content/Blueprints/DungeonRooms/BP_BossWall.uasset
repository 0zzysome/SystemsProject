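; BP_BossWall is a dungeon room barrier tied to a referenced boss that appears while the boss fight is on.
; On BeginPlay it hides its static mesh and disables collision, then, if the boss reference is valid, binds to that boss's events.
; Boss activation makes the wall visible and solid, and the death event from the boss's health component destroys the wall.
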(event `self.ReceiveBeginPlay`
  (bind _staticmesh1 (`self.StaticMesh1`))
  ;[1 1 1] Hide wall on start
  (`PrimitiveComponent.SetCollisionEnabled` _staticmesh1 "NoCollision")
  (`SceneComponent.SetVisibility` _staticmesh1 false false)
  ;[1 1 1] Activate wall once boss is enabled
  (bind _bossrefrence (`self.BossRefrence`)
    (:`then`
      (add `/Game/Blueprints/Enemies/BP_BossBase.BossActivated` _bossrefrence (delegate `EnableWall`))
      ;[1 1 1] Destroy self if boss is dead
      (add `/Game/Blueprints/BP_HealthComponent.HasDied` (`/Game/Blueprints/Enemies/BP_BossBase.BP_HealthComponent` _bossrefrence) (delegate `HasDied`)))
    (:`else`)))

(event `HasDied`
  ;[1 1 1] Destroy self if boss is dead
  (`self.K2_DestroyActor`))

(event `EnableWall`
  (bind _staticmesh1 (`self.StaticMesh1`))
  ;[1 1 1] Activate wall once boss is enabled
  (`PrimitiveComponent.SetCollisionEnabled` _staticmesh1 "QueryAndPhysics")
  (`SceneComponent.SetVisibility` _staticmesh1 true false))

(fn `UserConstructionScript`)