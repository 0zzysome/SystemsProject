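; BP_WeaponDamageUP is a loot pickup that upgrades the damage of the player's weapon.
; On its Pickup event it checks that the player's BPWeaponComponent is valid, calls ImproveDamage with its UpgradeAmount, then destroys itself.
; If the component is invalid, nothing happens and the pickup stays; its BeginPlay, overlap and Tick events are unused.
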(event `/Game/Blueprints/BP_PickupInterface.Pickup`
  (params (PlayerRef :type "/Game/Blueprints/BP_MainCharacter Object Reference"))
  (bind _bp_weaponcomponent (`/Game/Blueprints/BP_MainCharacter.BP_WeaponComponent` PlayerRef)
    (:`then`
      (`/Game/Blueprints/BP_WeaponComponent.ImproveDamage` _bp_weaponcomponent (`self.UpgradeAmount`))
      (`self.K2_DestroyActor`))
    (:`else`)))

(fn `UserConstructionScript`
  (`parent.UserConstructionScript`))