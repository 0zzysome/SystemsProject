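; Base pickup actor that shows a title and description info box while a player overlaps it.
; BeginPlay creates a WBP_PickupInfo widget, assigns it to the InfoBox component and hides it.
; OverlappedPickup shows the widget and starts a looping timer that turns it toward the player's camera; StopOverlappedPickup hides it and clears the timer.
; The fast per-pickup timer is flagged as a possible performance cost when many run at once.
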(event `self.ReceiveBeginPlay`
  ;[0 1 0.1032] Widget setup
  (bind _returnvalue (`|CreateWidget` "/Game/UI/WBP_PickupInfo.WBP_PickupInfo_C" null (`self.Title`) (`self.Description`)))
  (bind _output_get (set `self.InfoBoxWidget` _returnvalue))
  (`WidgetComponent.SetWidget` (`self.InfoBox`) _output_get)
  (`Widget.SetVisibility` (`self.InfoBoxWidget`) "Hidden"))

(event `/Game/Blueprints/BP_PickupInterface.OverlappedPickup`
  (params (PlayerRef :type "/Game/Blueprints/BP_MainCharacter Object Reference"))
  ;[0 1 0.1032] Makes widget visible and face player (Warning: too many of these timers may create performance issues)
  (set `self.Player Ref` PlayerRef)
  (if (not (`KismetSystemLibrary.K2_IsValidTimerHandle` (`self.WidgetFaceingTick`)))
    (bind _returnvalue (`KismetSystemLibrary.K2_SetTimerDelegate` (delegate `RotateWidgetToCamera`) 0.01 true true))
    (set `self.WidgetFaceingTick` _returnvalue)
    (`Widget.SetVisibility` (`self.InfoBoxWidget`) "Visible")))

(event `RotateWidgetToCamera`
  (bind _infobox (`self.InfoBox`))
  ;[0 1 0.1032] Makes widget visible and face player (Warning: too many of these timers may create performance issues)
  (`SceneComponent.K2_SetWorldRotation` _infobox (`KismetMathLibrary.FindLookAtRotation` (`SceneComponent.K2_GetComponentLocation` _infobox) (`SceneComponent.K2_GetComponentLocation` (`/Game/Blueprints/BP_MainCharacter.Camera` (`self.Player Ref`)))) false false))

(event `/Game/Blueprints/BP_PickupInterface.StopOverlappedPickup`
  (bind _widgetfaceingtick (`self.WidgetFaceingTick`))
  ;[0 1 0.1032] Comment
  (`Widget.SetVisibility` (`self.InfoBoxWidget`) "Hidden")
  (if (`KismetSystemLibrary.K2_IsValidTimerHandle` _widgetfaceingtick)
    (`KismetSystemLibrary.K2_ClearAndInvalidateTimerHandle` _widgetfaceingtick)))

(fn `UserConstructionScript`)