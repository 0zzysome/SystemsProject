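; BP_WeaponBase is a base weapon Blueprint that deals damage to actors it touches.
; When its DamageCollision component begins overlapping an actor other than its owner, it checks that actor for BP_DamageInterface and sends DealDamageMessage with its Damage value.
; On BeginPlay it prints its owner's name as debug output.
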(event `self.ReceiveBeginPlay`
  (`KismetSystemLibrary.PrintString` (`KismetStringLibrary.Concat_StrStr` "OWNER: " (`KismetSystemLibrary.GetDisplayName` (`self.GetOwner`)))))

(event `self.DamageCollision.OnComponentBeginOverlap`
  (params (OverlappedComponent :type "PrimitiveComponent Object Reference") (OtherActor :type "Actor Object Reference") (OtherComp :type "PrimitiveComponent Object Reference") (OtherBodyIndex :type Integer) (bFromSweep :type Boolean) (SweepResult :type "HitResult Structure (by ref)"))
  (if (not (== OtherActor (`self.GetOwner`)))
    (if (`KismetSystemLibrary.DoesImplementInterface` OtherActor "/Game/Blueprints/BP_DamageInterface.BP_DamageInterface_C")
      (message `/Game/Blueprints/BP_DamageInterface.DealDamage` OtherActor (`self.Damage`)))))

(fn `UserConstructionScript`)