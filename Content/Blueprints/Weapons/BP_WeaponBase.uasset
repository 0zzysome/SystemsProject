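; Base weapon actor that can be picked up, equips through the player's weapon component, and damages overlapped non-owner actors via BP_DamageInterface.
; The construction script sizes the damage capsule from Range and enables pickup collision only while unequipped.
; A world-space info widget shows type and stats, refreshed by the stat update events.
; During pickup overlap, a looping timer, rather than Tick, turns the widget toward the player's camera.
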(event `self.ReceiveBeginPlay`
  (bind _weaponinfowidget (`self.WeaponInfoWidget`))
  ;[0 1 0.1032] Create info widget
  (bind _returnvalue (`|CreateWidget` "/Game/UI/WBP_WeaponInfo.WBP_WeaponInfo_C"))
  (bind _output_get (set `self.WeaponInfoWidget` _returnvalue))
  (`WidgetComponent.SetWidget` (`self.Widget`) _output_get)
  (`Widget.SetVisibility` _output_get "Hidden")
  (`/Game/UI/WBP_WeaponInfo.UpdateStatsText` _weaponinfowidget (`self.Damage`) (`self.Range`) (`self.AttackSpeed`))
  (`/Game/UI/WBP_WeaponInfo.UpdateWeaponType` _weaponinfowidget (`self.WeaponTypeText`)))

(event `self.DamageCollision.OnComponentBeginOverlap`
  (params (OverlappedComponent :type "PrimitiveComponent Object Reference") (OtherActor :type "Actor Object Reference") (OtherComp :type "PrimitiveComponent Object Reference") (OtherBodyIndex :type Integer) (bFromSweep :type Boolean) (SweepResult :type "HitResult Structure (by ref)"))
  (if (not (== OtherActor (`self.GetOwner`)))
    (if (`KismetSystemLibrary.DoesImplementInterface` OtherActor "/Game/Blueprints/BP_DamageInterface.BP_DamageInterface_C")
      (message `/Game/Blueprints/BP_DamageInterface.DealDamage` OtherActor (`self.Damage`)))))

(event `UpdateDamage`
  (params (Damage :type "Float (double-precision)"))
  ;[1 1 1] Update stats for later
  (set `self.Damage` Damage)
  ;[1 1 1] Update the text also
  (`/Game/UI/WBP_WeaponInfo.UpdateStatsText` (`self.WeaponInfoWidget`) (`self.Damage`) (`self.Range`) (`self.AttackSpeed`) :!label _label))

(event `UpdateRange`
  (params (Range :type "Float (double-precision)"))
  ;[1 1 1] Update stats for later
  (set `self.Range` Range)
  (goto _label))

(event `UpdateAttackSpeed`
  (params (AttackSpeed :type "Float (double-precision)"))
  ;[1 1 1] Update stats for later
  (set `self.AttackSpeed` AttackSpeed)
  (goto _label))

(event `/Game/Blueprints/BP_PickupInterface.Pickup`
  (params (PlayerRef :type "/Game/Blueprints/BP_MainCharacter Object Reference"))
  ;[1 1 1] Equip weapon when picked up.
  (if (not (`self.IsEquiped?`))
    (`/Game/Blueprints/BP_WeaponComponent.EquipNewWeapon` (`/Game/Blueprints/BP_MainCharacter.BP_WeaponComponent` PlayerRef) self)
    (if (`KismetSystemLibrary.K2_IsValidTimerHandle` (`self.WidgetFaceingTick`))
      (`self.HideWidget`))))

(event `/Game/Blueprints/BP_PickupInterface.OverlappedPickup`
  (params (PlayerRef :type "/Game/Blueprints/BP_MainCharacter Object Reference"))
  ;[0 1 0.1032] Makes widget visible and face player (Warning: too many of these timers may create performance issues)
  (set `self.Player Ref` PlayerRef)
  (if (not (`self.IsEquiped?`))
    (if (not (`KismetSystemLibrary.K2_IsValidTimerHandle` (`self.WidgetFaceingTick`)))
      (bind _returnvalue (`KismetSystemLibrary.K2_SetTimerDelegate` (delegate `RotateWidgetToCamera`) 0.01 true true))
      (set `self.WidgetFaceingTick` _returnvalue)
      (`Widget.SetVisibility` (`self.WeaponInfoWidget`) "HitTestInvisible"))))

(event `RotateWidgetToCamera`
  (bind _widget (`self.Widget`))
  ;[0 1 0.1032] Makes widget visible and face player (Warning: too many of these timers may create performance issues)
  (`SceneComponent.K2_SetWorldRotation` _widget (`KismetMathLibrary.FindLookAtRotation` (`SceneComponent.K2_GetComponentLocation` _widget) (`SceneComponent.K2_GetComponentLocation` (`/Game/Blueprints/BP_MainCharacter.Camera` (`self.Player Ref`)))) false false))

(event `HideWidget`
  ;[0 1 0.1032] Hides Widget
  (`Widget.SetVisibility` (`self.WeaponInfoWidget`) "Hidden")
  (`KismetSystemLibrary.K2_ClearAndInvalidateTimerHandle` (`self.WidgetFaceingTick`)))

(event `/Game/Blueprints/BP_PickupInterface.StopOverlappedPickup`
  ;[0 1 0.1032] When player leaves pickup range.
  (`self.HideWidget`))

(fn `UserConstructionScript`
  (bind _range (`self.Range`))
  (bind _damagecollision (`self.DamageCollision`))
  (bind _pickupcollision (`self.PickupCollision`))
  (`SceneComponent.K2_SetRelativeLocation` _damagecollision (`KismetMathLibrary.MakeVector` 0.0 0.0 _range) false false)
  (`CapsuleComponent.SetCapsuleHalfHeight` _damagecollision _range true)
  (if (`self.IsEquiped?`)
    (`PrimitiveComponent.SetCollisionEnabled` _pickupcollision "NoCollision")
    (else
      (`PrimitiveComponent.SetCollisionEnabled` _pickupcollision "QueryOnly"))))