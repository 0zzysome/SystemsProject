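; BP_EnemySpawnComponent spawns AI enemies at its child components' transforms shortly after BeginPlay.
; When spawning is enabled, the count is either fixed or random between a minimum and maximum.
; Each spawn takes a random class from EnemiesToSpawn and fills child points in index order rather than randomly.
; Debug messages report when child points are missing or too few for the requested count.
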(event `self.ReceiveBeginPlay`
  (bind _returnvalue (`KismetMathLibrary.RandomIntegerInRange` (`self.MinSpawnAmount`) (`self.SpawnEnemyAmount`)))
  ;[1 1 1] Enshure variables are in order
  (`KismetSystemLibrary.Delay` 0.2)
  (set `self.SpawnLocations` (`self.GetChildrenComponents` false))
  (if (`KismetArrayLibrary.Array_IsNotEmpty` (`self.SpawnLocations`))
    (if (`KismetArrayLibrary.Array_IsNotEmpty` (`self.Enemies To Spawn `))
      (if (`self.bShouldSpawnEnemies?`)
        (if (`self.bShouldRandomSpawn`)
          ;[1 1 1] Get a random number over 0
          (if (not (<= _returnvalue 0))
            (for _index (range _returnvalue)
              (bind _output (`|GetArrayItem` (`self.SpawnLocations`) _index))
              ;[1 1 1] spawn enemies
              (`/Engine/EditorBlueprintResources/StandardMacros.IsValid` _output
                (:`Is Valid`
                  (`AIBlueprintHelperLibrary.SpawnAIFromClass` (`KismetArrayLibrary.Array_Random` (`self.Enemies To Spawn `)) null (`self.K2_GetComponentLocation` _output) (`self.K2_GetComponentRotation` _output) false null))
                (:`Is Not Valid`
                  (`KismetSystemLibrary.PrintString` (`KismetStringLibrary.Concat_StrStr` "NOT ENOUGHT SPAWN POINTS TO SPAWN ENEMY IN: " (`KismetSystemLibrary.GetDisplayName` (`self.GetOwner`))) :!label _label)))))
          (else
            (for _index_2 (range (`self.SpawnEnemyAmount`))
              (bind _output_2 (`|GetArrayItem` (`self.SpawnLocations`) _index_2))
              ;[1 1 1] Spawn enemies
              (`/Engine/EditorBlueprintResources/StandardMacros.IsValid` _output_2
                (:`Is Valid`
                  (`AIBlueprintHelperLibrary.SpawnAIFromClass` (`KismetArrayLibrary.Array_Random` (`self.Enemies To Spawn `)) null (`self.K2_GetComponentLocation` _output_2) (`self.K2_GetComponentRotation` _output_2) false null))
                (:`Is Not Valid`
                  (goto _label))))))))
    (else
      (`KismetSystemLibrary.PrintString` "NO CHILDREN COMPINENTS FOUND FOR SPAWN POINTS"))))