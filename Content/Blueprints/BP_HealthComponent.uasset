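; Health component shared by the main character and enemies, tracking current and max health and calling HasDied at zero.
; BeginPlay casts the owner to pick a viewport health bar for the player or an initially hidden widget-component bar for enemies.
; Damage passes through a DoOnce that reopens after InvulnTime, giving invulnerability frames, then clamps to max and refreshes the matching widget.
; Max health bonuses also heal by the added amount.
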(event `self.ReceiveBeginPlay`
  ;[1 1 1] Player
  (`|ExecutionSequence`
    (:`then_0`
      (bind _asbp_main_character (cast `/Game/Blueprints/BP_MainCharacter` (`self.GetOwner`)))
      (set `self.As BP Main Character` _asbp_main_character)
      (set `self.bIsPlayer` true)
      (bind _returnvalue (`|CreateWidget` "/Game/UI/WBP_PlayerHealth.WBP_PlayerHealth_C" (`GameplayStatics.GetPlayerController` 0)))
      (bind _output_get (set `self.PlayerHeathRef` _returnvalue))
      (`UserWidget.AddToViewport` _output_get 0)
      (`/Game/UI/WBP_PlayerHealth.UpdateHealth` _output_get (`self.CurrentHealth`) (`self.MaxHealth`)))
    (:`then_1`
      ;[1 1 1] Enemy
      (bind _asbp_enemy_base (cast `/Game/Blueprints/Enemies/BP_EnemyBase` (`self.GetOwner`)))
      (bind _output_get_2 (set `self.As BP Enemy Base` _asbp_enemy_base))
      (set `self.bIsPlayer` false)
      (bind _output_get_3 (set `self.Enemy health widget` (`/Game/Blueprints/Enemies/BP_EnemyBase.HealthWidget` _output_get_2)))
      (`/Engine/EditorBlueprintResources/StandardMacros.IsValid` _output_get_3
        (:`Is Valid`
          (bind _returnvalue_2 (`|CreateWidget` "/Game/UI/WBP_EnemyHealth.WBP_EnemyHealth_C"))
          (bind _output_get_4 (set `self.Enemyhealth` _returnvalue_2))
          (`WidgetComponent.SetWidget` _output_get_3 _output_get_4)
          (`/Game/UI/WBP_EnemyHealth.UpdateHp` _output_get_4 (`self.CurrentHealth`) (`self.MaxHealth`))
          (`Widget.SetVisibility` _output_get_4 "Hidden"))
        (:`Is Not Valid`
          (`KismetSystemLibrary.PrintString` "WIDGET COMPONENT IS NOT SET FOR ENEMY"))))))

(event `TakeDamageEvent`
  (params (Damage :type "Float (double-precision)"))
  ;[1 1 1] Take damage
  (`/Engine/EditorBlueprintResources/StandardMacros.DoOnce` false :!label _label
    (:`Completed`
      (bind _output_get (set `self.CurrentHealth` (- (`self.CurrentHealth`) Damage))) ; update current health
      (if (>= _output_get (`self.MaxHealth`))
        (set `self.CurrentHealth` (`self.MaxHealth`))
        (`self.UpdateHealthToWidget`)
        (elif (<= (`self.CurrentHealth`) 0.0)
          (`self.UpdateHealthToWidget`)
          (`self.HasDied`)
          (else
            (`self.UpdateHealthToWidget`))))
      (`KismetSystemLibrary.Delay` (`self.InvulnTime`))
      (`self.RemoveInvulnFrames`))))

(event `RemoveInvulnFrames`
  ;[1 1 1] Take damage
  (goto _label :!via `Reset`))

(event `UpdatemaxhealthEvent`
  (params (AddedMaxHealth :type "Float (double-precision)"))
  ;[1 1 1] Add max health bonus to total
  (set `self.MaxHealth` (+ (`self.MaxHealth`) AddedMaxHealth))
  ;[1 1 1] heal that amount
  (set `self.CurrentHealth` (+ (`self.CurrentHealth`) AddedMaxHealth))
  (`self.UpdateHealthToWidget`))

(fn `UpdateHealthToWidget`
  (if (`self.bIsPlayer`)
    (`/Game/UI/WBP_PlayerHealth.UpdateHealth` (`self.PlayerHeathRef`) (`self.CurrentHealth`) (`self.MaxHealth`))
    (else
      (`/Game/UI/WBP_EnemyHealth.UpdateHp` (`self.Enemyhealth`) (`self.CurrentHealth`) (`self.MaxHealth`)))))